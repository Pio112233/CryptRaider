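; Dungeon doorway actor with left and right door meshes that swing open when its OpenDoor event is called.
; OpenDoor plays the DoorAnim timeline from the start, lerping each door's relative rotation toward its own target yaw by the timeline alpha.
; Each lerp starts from the door's current rotation rather than a cached one, so the motion compounds per update.
; The Blueprint has no close logic or trigger of its own.
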(event Custom|OpenDoor
  (bind _alpha (Timeline|DoorAnim PlayFromStart)
    (:Update
      (Transformation|SetRelativeRotation (Variables|Default|GetSM_DoorWay_Large_Door_Left) (Math|Rotator|Lerp(Rotator) (Variables|/Script/Engine.SceneComponent|GetRelativeRotation (Variables|Default|GetSM_DoorWay_Large_Door_Left)) (Math|Rotator|MakeRotator 0.0 0.0 (Variables|Default|GetLeftDoorTargetYaw)) _alpha) false false)
      (Transformation|SetRelativeRotation (Variables|Default|GetSM_DoorWay_Large_Door_Right) (Math|Rotator|Lerp(Rotator) (Variables|/Script/Engine.SceneComponent|GetRelativeRotation (Variables|Default|GetSM_DoorWay_Large_Door_Right)) (Math|Rotator|MakeRotator 0.0 0.0 (Variables|Default|GetRightDoorTargetYaw)) _alpha) false false))))

(event EventBeginPlay
  (|CallParentFunction) ; This node is disabled and will not be called.\nDrag off pins to build functionality.
)

(event Collision|EventActorBeginOverlap
  (params (OtherActor :type Actor%20Object%20Reference))
  (|CallParentFunction OtherActor) ; This node is disabled and will not be called.\nDrag off pins to build functionality.
)

(event EventTick
  (params (DeltaSeconds :type Float%20%28single-precision%29))
  (|CallParentFunction DeltaSeconds) ; This node is disabled and will not be called.\nDrag off pins to build functionality.
)

(fn ConstructionScript
  (|CallParentFunction))