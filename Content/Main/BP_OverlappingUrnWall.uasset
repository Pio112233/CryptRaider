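; Urn wall puzzle actor that tests whether a connected wall's collider has a component inside it.
; An overlap event from its WallBoxComponent calls CheckPuzzleProgress, which returns whether that collider's ComponentInside is valid.
; The event graph does not use the returned result, and Tick and construction only call their parent versions.
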(event OnSupportedCompOverlap(WallBoxComponent)
  (params (Component :type Primitive%20Component%20Object%20Reference))
  (CallFunction|CheckPuzzleProgress))

(event EventBeginPlay
  (|CallParentFunction) ; This node is disabled and will not be called.\nDrag off pins to build functionality.
)

(event Collision|EventActorBeginOverlap
  (params (OtherActor :type Actor%20Object%20Reference))
  (|CallParentFunction OtherActor) ; This node is disabled and will not be called.\nDrag off pins to build functionality.
)

(event EventTick
  (params (DeltaSeconds :type Float%20%28single-precision%29))
  (|CallParentFunction DeltaSeconds))

(fn ConstructionScript
  (|CallParentFunction))

(fn CheckPuzzleProgress
  (return (Utilities|IsValid (Variables|/Script/CryptRaider.WallBoxComponent|GetComponentInside (Class|OverlappingActor|GetCollider (Variables|Default|GetConnectedWall))))))