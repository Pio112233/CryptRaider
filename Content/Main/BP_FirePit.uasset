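; BP_FirePit is a fire pit trigger that activates its particle system and sets a linked door moving.
; The WallBoxComponent's OnSupportedCompOverlap event drives it through a DoOnce, so the reaction fires a single time.
; The door opens through a Mover component looked up on DoorRef, which receives SetShouldMove only if that component is valid.
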(event OnSupportedCompOverlap(WallBoxComponent)
  (params (Component :type Primitive%20Component%20Object%20Reference))
  (bind _doorref (Variables|Default|GetDoorRef))
  (bind _returnvalue (Actor|GetComponentbyClass _doorref "/Script/CryptRaider.Mover"))
  (Utilities|FlowControl|DoOnce false
    (:Completed
      (Components|Activation|Activate (Variables|Default|GetParticleSystem) true)
      (Utilities|IsValid _returnvalue
        (:Is%20Valid
          (Class|Mover|SetShouldMove _returnvalue true))))))

(event EventBeginPlay
  (|CallParentFunction))

(event Collision|EventActorBeginOverlap
  (params (OtherActor :type Actor%20Object%20Reference))
  (|CallParentFunction OtherActor) ; This node is disabled and will not be called.\nDrag off pins to build functionality.
)

(event EventTick
  (params (DeltaSeconds :type Float%20%28single-precision%29))
  (|CallParentFunction DeltaSeconds) ; This node is disabled and will not be called.\nDrag off pins to build functionality.
)

(fn ConstructionScript
  (|CallParentFunction))